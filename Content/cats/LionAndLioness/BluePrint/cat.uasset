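; Cat actor that shows the score and handles the win condition for a cheese-collecting goal.
; Every Tick creates a new Score widget and adds it to the viewport, with no reuse or removal of earlier ones.
; When CheeseCount reaches Goal, it adds the GameWon widget, shows the mouse cursor and destroys itself.
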(event `self.ReceiveTick`
  (params (DeltaSeconds :type "Float (single-precision)"))
  (bind _returnvalue (`|CreateWidget` "/Game/ThirdPersonCPP/Maps/Score.Score_C"))
  (`UserWidget.AddToViewport` _returnvalue 0)
  (if (>= (`self.Cheese_count`) (`self.goal`))
    (bind _returnvalue_2 (`|CreateWidget` "/Game/ThirdPersonCPP/Mouse/GameWon_Widget.GameWon_Widget_C"))
    (`UserWidget.AddToViewport` _returnvalue_2 0)
    (set `PlayerController.bShowMouseCursor` true (`GameplayStatics.GetPlayerController` 0))
    (`self.K2_DestroyActor`)))

(fn `UserConstructionScript`)