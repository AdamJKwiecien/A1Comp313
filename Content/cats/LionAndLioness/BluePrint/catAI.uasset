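; Lion/lioness cat AI actor that wanders at random and ends the game when it touches the player.
; Tick uses a random Delay to pace AI moves to nearby reachable points, toggling IsMoving around each move.
; A Box overlap matched by display name to Char plays Cat_death, destroys the player character and itself, and shows the GameOver widget with the mouse cursor.
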(event `self.ReceiveTick`
  (params (DeltaSeconds :type "Float (single-precision)"))
  ;[1 1 1] Movement for cat
  (`KismetSystemLibrary.Delay` (`KismetMathLibrary.RandomFloatInRange` 1.0 6.0))
  (set `self.is Moving` true)
  (`|AIMoveTo` self (`NavigationSystemV1.K2_GetRandomReachablePointInRadius` (`self.K2_GetActorLocation`) 500.0 null null) null
    (:`OnSuccess`
      _)
    (:`OnFail`
      _))
  (set `self.is Moving` false))

(event `self.Box.OnComponentBeginOverlap`
  (params (OverlappedComponent :type "PrimitiveComponent Object Reference") (OtherActor :type "Actor Object Reference") (OtherComp :type "PrimitiveComponent Object Reference") (OtherBodyIndex :type Integer) (bFromSweep :type Boolean) (SweepResult :type "HitResult Structure (by ref)"))
  (if (`KismetStringLibrary.EqualEqual_StrStr` (`KismetSystemLibrary.GetDisplayName` OtherActor) (`self.char`))
    (`GameplayStatics.PlaySound2D` "/Game/ThirdPersonCPP/Cheese/cat_death.cat_death" 1.0 1.0 0.0 null null)
    (bind _asthird_person_character (cast `/Game/ThirdPersonCPP/Blueprints/ThirdPersonCharacter` (`GameplayStatics.GetPlayerPawn` 0)))
    (`self.K2_DestroyActor` _asthird_person_character)
    (bind _returnvalue (`|CreateWidget` "/Game/ThirdPersonCPP/Maps/GameOver.GameOver_C"))
    (`UserWidget.AddToViewport` _returnvalue 0)
    (set `PlayerController.bShowMouseCursor` true (`GameplayStatics.GetPlayerController` 0))
    (`self.K2_DestroyActor`)))

(fn `UserConstructionScript`)